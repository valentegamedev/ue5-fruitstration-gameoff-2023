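; Game mode that runs a timed fruit-order game, advancing through a list of orders and handling retry and game over.
; Fruits added or removed trigger matching by type and volume within a weight-relative tolerance, and a session advances once every order entry matches.
; A looping timer scaled to order size updates the HUD, fires a one-shot camera shake and level sequence warning when low, then ends the game.
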(event Custom|StartTimer
  (bind _almostoversequence (Variables|Default|GetAlmostOverSequence))
  (bind _sequenceplayer (Variables|/Script/LevelSequence.LevelSequenceActor|GetSequencePlayer _almostoversequence))
  (CallFunction|StopTimer)
  (if (not (Variables|Default|GetbIsGameOver))
    (bind _order (CallFunction|GetCurrentOrder))
    (Variables|Default|SetTimerCounter (* (Utilities|Array|Length (.orderlist _order)) (.timeperfruit _order)))
    (bind _returnvalue (Utilities|Time|SetTimerbyEvent (delegate Custom|TimerEvent) 1.0 true))
    (Variables|Default|SetTimerHandle _returnvalue)
    (CallFunction|TimerEvent)
    (Utilities|FlowControl|DoOnce false) ; enters at Reset
  ))

(event Custom|TimerEvent
  (if (== (Variables|Default|GetTimerCounter) -1)
    (CallFunction|EndGame)
    (else
      (bind _hud (CallFunction|GetCastedHUD))
      (Default|UpdateTime (Variables|/Game/Blueprints/GameplayFramework/BP_HUD.BP_HUD_C|GetHUD _hud) (Variables|Default|GetTimerCounter))
      (bind _result (Math|Integer|DecrementInt (Variables|Default|GetTimerCounter))
        (:%20%20
          (if (<= _result (Variables|Default|GetAlmostOverTime))
            (CallFunction|AlmostOverEvent)))))))

(event Custom|StopTimer
  (Utilities|Time|ClearandInvalidateTimerbyHandle (Variables|Default|GetTimerHandle))
  (Sequencer|Player|Stop (Variables|/Script/LevelSequence.LevelSequenceActor|GetSequencePlayer (Variables|Default|GetAlmostOverSequence)) :!class /Script/MovieScene.MovieSceneSequencePlayer)
  (CameraShake|StopAllCameraShakes (Game|GetPlayerCameraManager 0) true))

(event Custom|AlmostOverEvent
  (bind _almostoversequence (Variables|Default|GetAlmostOverSequence))
  (bind _sequenceplayer (Variables|/Script/LevelSequence.LevelSequenceActor|GetSequencePlayer _almostoversequence))
  (Utilities|FlowControl|DoOnce false
    (:Completed
      (CameraShakes|StartCameraShake (Game|GetPlayerCameraManager 0) "/Game/Blueprints/BP_CameraShakeAlmostOver.BP_CameraShakeAlmostOver_C" 2.0 "CameraLocal" "0, 0, 0")
      (Components|Timeline|SetPlaybackPosition _sequenceplayer (Utilities|Struct|MakeMovieSceneSequencePlaybackParams "(FrameNumber=(Value=0),SubFrame=0.000000)" 0.0 "" "Frame" "Play" false))
      (Sequencer|Player|Play _sequenceplayer :!class /Script/MovieScene.MovieSceneSequencePlayer)
      (bind _hud (CallFunction|GetCastedHUD))
      (Default|HideRetryButton (Variables|/Game/Blueprints/GameplayFramework/BP_HUD.BP_HUD_C|GetHUD _hud)))))

(event EventBeginPlay
  (bind _outactor (Sequencer|Player|CreateLevelSequencePlayer "/Game/Sequences/AlmostOverLevelSequence.AlmostOverLevelSequence" (Utilities|Struct|MakeMovieSceneSequencePlaybackSettings false "(Value=0)" 0.7 0.0 false false false false false false false true)))
  (Variables|Default|SetAlmostOverSequence _outactor)
  (bind _returnvalue (Audio|SpawnSound2D "/Game/Sounds/SC_BackgroundMusic.SC_BackgroundMusic" 1.0 1.0 0.0 0))
  (bind _output_get (Variables|Default|SetBackgroundMusic _returnvalue))
  (Audio|Components|Audio|SetVolumeMultiplier _output_get 0.6 :!class /Script/Engine.AudioComponent))

(fn ConstructionScript)

(fn GetCurrentOrder
  (bind _orderindex (Variables|Default|GetOrderIndex))
  (return (Utilities|Array|Get(acopy) (Variables|Default|GetOrderList) _orderindex) _orderindex))

(fn Initialize
  (bind _order (CallFunction|GetCurrentOrder))
  (bind _outactors (Actor|GetAllActorsOfClasswithTag "/Script/Engine.TargetPoint" "FruitSpawner"))
  (if (> (Utilities|Array|Length _outactors) 0)
    (Game|SpawnActorfromClass (.fruitspawner _order) (Transformation|GetActorTransform (Utilities|Array|Get(acopy) _outactors)) "Undefined" "MultiplyWithRoot" 0 0)))

(fn ProcessOrder
  (if (not (Variables|Default|GetbIsGameOver))
    (Utilities|FlowControl|Sequence
      (:then_0
        (Utilities|Array|Clear (Variables|Default|GetCheckedIndexes))
        (Utilities|Array|Clear (LocalVariables|GetUsedItems))
        (bind _order (CallFunction|GetCurrentOrder))
        (for (_array_element _array_index) (.orderlist _order)
          (bind _output_get (LocalVariables|SetOrderTolerance (* (.weight _array_element) (Variables|Default|GetTolerance))))
          (bind (_array_element_2 _array_index_2) (Utilities|Array|ForEachLoopwithBreak (Variables|Default|GetFruitsInOrder) :!label _label)
            (:LoopBody
              (if (== (.fruitdata _array_element) (Variables|/Script/Fruitstration.VFruit|GetFruitData _array_element_2))
                (bind _returnvalue (Class|VFruit|GetVolume _array_element_2))
                (if (< (Math|Float|Absolute(Float) (- (.weight _array_element) _returnvalue)) _output_get)
                  (if (not (Utilities|Array|ContainsItem (LocalVariables|GetUsedItems) _array_index_2))
                    (Utilities|Array|Add (Variables|Default|GetCheckedIndexes) _array_index)
                    (Utilities|Array|AddUnique (LocalVariables|GetUsedItems) _array_index_2)
                    (goto _label Break)))))))))))

(fn AddtoOrder
  (params (Fruit :type BP%20Fruit%20Object%20Reference))
  (Utilities|Array|AddUnique (Variables|Default|GetFruitsInOrder) Fruit)
  (CallFunction|ProcessOrder))

(fn RemovefromOrder
  (params (Fruit :type BP%20Fruit%20Object%20Reference))
  (Utilities|Array|RemoveItem (Variables|Default|GetFruitsInOrder) Fruit)
  (CallFunction|ProcessOrder))

(fn GetCheckedIndexes
  (return (Variables|Default|GetCheckedIndexes)))

(fn EndSession
  (bind _checkedindexes (CallFunction|GetCheckedIndexes))
  (bind _order (CallFunction|GetCurrentOrder))
  (if (== (Utilities|Array|Length _checkedindexes) (Utilities|Array|Length (.orderlist _order)))
    (bind _result (Math|Integer|IncrementInt (Variables|Default|GetOrderIndex))
      (:%20%20
        (bind _output_get (Variables|Default|SetbIsGameOver (== _result (Utilities|Array|Length (Variables|Default|GetOrderList)))))
        (if _output_get
          (bind _hud (CallFunction|GetCastedHUD))
          (Default|HideAll (Variables|/Game/Blueprints/GameplayFramework/BP_HUD.BP_HUD_C|GetHUD _hud)))
        (CallFunction|StopTimer))))
  (return (== (Utilities|Array|Length _checkedindexes) (Utilities|Array|Length (.orderlist _order)))))

(fn IsGameOver
  (return (Variables|Default|GetbIsGameOver)))

(fn EndGame
  (Utilities|Time|ClearandInvalidateTimerbyHandle (Variables|Default|GetTimerHandle))
  (Sequencer|Player|Pause (Variables|/Script/LevelSequence.LevelSequenceActor|GetSequencePlayer (Variables|Default|GetAlmostOverSequence)))
  (CameraShake|StopAllCameraShakes (Game|GetPlayerCameraManager 0) true)
  (bind _hud (CallFunction|GetCastedHUD))
  (Default|ShowEndGame (Variables|/Game/Blueprints/GameplayFramework/BP_HUD.BP_HUD_C|GetHUD _hud))
  (Audio|PlaySound2D "/Game/Sounds/SC_GameOver.SC_GameOver" 6.0 1.0 0.0 0 0)
  (Audio|Components|Audio|Stop (Variables|Default|GetBackgroundMusic)))

(fn RetrySession
  (CallFunction|StopTimer)
  (Variables|Default|SetbIsGameOver false)
  (bind _outactors (Actor|GetAllActorsOfClass "/Game/Blueprints/BP_Fruit.BP_Fruit_C"))
  (for _array_element _outactors
    (Actor|DestroyActor _array_element))
  (bind _outactors_2 (Actor|GetAllActorsOfClass "/Game/Blueprints/BP_Decal.BP_Decal_C"))
  (for _array_element_2 _outactors_2
    (Actor|DestroyActor _array_element_2))
  (CallFunction|Initialize))