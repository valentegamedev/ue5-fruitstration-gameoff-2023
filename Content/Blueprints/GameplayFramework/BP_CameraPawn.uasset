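; Player camera pawn for a fruit-cutting game, turning mouse input into fruit dragging, blade cuts and widget clicks.
; Tick traces under the cursor to track the hovered fruit, show a grab cursor and aim the WidgetInteraction component.
; Pressing on fruit drags it with physics off across board, scale and table.
; Pressing on the cutting board starts a spawned BP_Blade cut, with blade position projected onto a fixed horizontal plane.
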(event Custom|StartGame
  (Utilities|FlowControl|Sequence
    (:then_0
      (Components|MoveComponentTo (Variables|Default|GetCameraComponent) "0, 0, 0" "0, 0, 0" true true 1.0 false))))

(event Custom|ReleaseClickEvent
  (bind _widgetinteraction (Variables|Default|GetWidgetInteraction))
  (Class|WidgetInteractionComponent|ReleasePointerKey _widgetinteraction "LeftMouseButton")
  (Class|WidgetInteractionComponent|ReleasePointerKey _widgetinteraction "RightMouseButton")
  (Class|VBlade|StopCut (Variables|Default|GetBlade))
  (Variables|Default|SetIsDragging false)
  (bind _fruitundermouse (Variables|Default|GetFruitUnderMouse)
    (:then
      (Physics|SetSimulatePhysics (Variables|/Script/GeometryFramework.DynamicMeshActor|GetDynamicMeshComponent _fruitundermouse) true)
      (Variables|Default|SetFruitUnderMouse 0))
    (:else)))

(event EventBeginPlay
  (Utilities|FlowControl|Sequence
    (:then_0
      (bind _returnvalue (Game|SpawnActorfromClass "/Game/Blueprints/BP_Blade.BP_Blade_C" (Math|Transform|MakeTransform "0, 0, 0" "0, 0, 0" "1.000000,1.000000,1.000000") "AlwaysSpawn" "MultiplyWithRoot" 0 self))
      (Variables|Default|SetBlade _returnvalue))))

(event EventTick
  (params (DeltaSeconds :type Float%20%28single-precision%29))
  (bind _returnvalue (Game|GetPlayerController 0))
  (bind _returnvalue_2 (Game|GetPlayerController 0))
  (bind _returnvalue_3 (Game|GetPlayerController 0))
  (bind _returnvalue_4 (Game|GetPlayerController 0))
  (bind (_worldlocation _worlddirection) (Game|Player|ConvertMouseLocationToWorldSpace _returnvalue))
  (bind (_locationx _locationy) (Game|Player|GetMousePosition _returnvalue_2))
  (bind (_locationx_2 _locationy_2) (Game|Player|GetMousePosition _returnvalue_3))
  (bind (_locationx_3 _locationy_3) (Game|Player|GetMousePosition _returnvalue_4))
  (bind (_worldposition _worlddirection_2) (Class|GameplayStatics|DeprojectScreentoWorld _returnvalue_2 (Math|Vector2D|MakeVector2D _locationx _locationy)))
  (bind (_worldposition_2 _worlddirection_3) (Class|GameplayStatics|DeprojectScreentoWorld _returnvalue_3 (Math|Vector2D|MakeVector2D _locationx_2 _locationy_2)))
  (bind (_worldposition_3 _worlddirection_4) (Class|GameplayStatics|DeprojectScreentoWorld _returnvalue_4 (Math|Vector2D|MakeVector2D _locationx_3 _locationy_3)))
  (Utilities|FlowControl|Sequence
    (:then_0
      (if (not (Variables|Default|GetIsDragging))
        (bind (_outhit _returnvalue_5) (Collision|LineTraceForObjects _worldposition_2 (+ _worldposition_2 (* _worlddirection_3 1e+03)) (Utilities|Array|MakeArray "ObjectTypeQuery2" "ObjectTypeQuery9" "ObjectTypeQuery10" "ObjectTypeQuery8") false 0 "None"))
        (if _returnvalue_5
          (bind _asbp_fruit (Utilities|Casting|CastToBP_Fruit (.hitactor _outhit))
            (:then
              (bind _fruitundermouse (Variables|Default|GetFruitUnderMouse)
                (:then
                  (if (!= _fruitundermouse _asbp_fruit)
                    (Variables|Default|SetFruitUnderMouse _asbp_fruit)
                    (Variables|/Script/Engine.PlayerController|SetCurrentMouseCursor (Game|GetPlayerController 0) "GrabHand" :!label _label)))
                (:else
                  (Variables|Default|SetFruitUnderMouse _asbp_fruit)
                  (goto _label))))
            (:CastFailed
              (Variables|Default|GetFruitUnderMouse :!label _label_2
                (:then
                  (Variables|/Script/Engine.PlayerController|SetCurrentMouseCursor (Game|GetPlayerController 0) "Default")
                  (Variables|Default|SetFruitUnderMouse 0))
                (:else))))
          (else
            (goto _label_2)))))
    (:then_1
      (Utilities|FlowControl|Gate true
        (:Exit
          (bind _blade (Variables|Default|GetBlade)
            (:then
              (Class|VBlade|UpdateLocation _blade (.Intersection (Class|KismetMathLibrary|LinePlaneIntersectionOriginNormal _worldlocation (+ _worldlocation (* _worlddirection 5e+03)) (Math|Vector|MakeVector -45.0 0.0 105.0) "0.000000,0.000000,1.000000"))))
            (:else)))))
    (:then_2
      (if (Variables|Default|GetIsDragging)
        (bind _fruitundermouse_2 (Variables|Default|GetFruitUnderMouse)
          (:then
            (bind (_outhit_2 _returnvalue_6) (Collision|LineTraceForObjects _worldposition (+ _worldposition (* _worlddirection_2 1e+04)) (Utilities|Array|MakeArray "ObjectTypeQuery8" "ObjectTypeQuery9" "ObjectTypeQuery10") false 0 "None"))
            (if _returnvalue_6
              (switch Utilities|FlowControl|Switch|SwitchonECollisionChannel (Collision|GetCollisionObjectType (.hitcomponent _outhit_2))
                (:ECC_GameTraceChannel2
                  _)
                (:ECC_GameTraceChannel3
                  _)
                (:ECC_GameTraceChannel4
                  _))
              (Transformation|SetActorLocation _fruitundermouse_2 (+ (.location _outhit_2) (Variables|Default|GetDragOffset)) false true)))
          (:else))))
    (:then_3
      (Transformation|SetWorldRotation (Variables|Default|GetWidgetInteraction) (Math|Rotator|FindLookatRotation _worldposition_3 (+ _worldposition_3 _worlddirection_4)) false false))))

(event Input|ActionEvents|InputActionInteract
  (params (Key :type Key%20Structure))
  (bind _returnvalue (Game|GetPlayerController 0))
  (bind _returnvalue_2 (Game|GetPlayerController 0))
  (bind _blade (Variables|Default|GetBlade))
  (bind _widgetinteraction (Variables|Default|GetWidgetInteraction))
  (bind (_locationx _locationy) (Game|Player|GetMousePosition _returnvalue_2))
  (bind (_worldlocation _worlddirection) (Game|Player|ConvertMouseLocationToWorldSpace _returnvalue))
  (bind (_worldposition _worlddirection_2) (Class|GameplayStatics|DeprojectScreentoWorld _returnvalue_2 (Math|Vector2D|MakeVector2D _locationx _locationy)))
  (:Pressed
    (Class|WidgetInteractionComponent|PressPointerKey _widgetinteraction "LeftMouseButton")
    (Class|WidgetInteractionComponent|PressPointerKey _widgetinteraction "RightMouseButton")
    (bind (_outhit _returnvalue_3) (Collision|LineTraceForObjects _worldposition (+ _worldposition (* _worlddirection_2 1e+04)) (Utilities|Array|MakeArray "ObjectTypeQuery8" "ObjectTypeQuery9" "ObjectTypeQuery10") false 0 "None"))
    (if _returnvalue_3
      (bind _fruitundermouse (Variables|Default|GetFruitUnderMouse)
        (:then
          (Variables|Default|SetIsDragging true)
          (Variables|Default|SetDragOffset (- (Transformation|GetActorLocation _fruitundermouse) (.location _outhit)))
          (Physics|SetSimulatePhysics (Variables|/Script/GeometryFramework.DynamicMeshActor|GetDynamicMeshComponent (Variables|Default|GetFruitUnderMouse)) false))
        (:else
          (switch Utilities|FlowControl|Switch|SwitchonECollisionChannel (Collision|GetCollisionObjectType (.hitcomponent _outhit))
            (:ECC_GameTraceChannel2
              (Class|VBlade|StartCut _blade (.location _outhit))
              (Utilities|FlowControl|Gate true) ; enters at Open
            ))))))
  (:Released
    (Class|WidgetInteractionComponent|ReleasePointerKey _widgetinteraction "LeftMouseButton")
    (Class|WidgetInteractionComponent|ReleasePointerKey _widgetinteraction "RightMouseButton")
    (Class|VBlade|StopCut _blade)
    (Variables|Default|SetIsDragging false)
    (bind _fruitundermouse_2 (Variables|Default|GetFruitUnderMouse)
      (:then
        (Physics|SetSimulatePhysics (Variables|/Script/GeometryFramework.DynamicMeshActor|GetDynamicMeshComponent _fruitundermouse_2) true)
        (Variables|Default|SetFruitUnderMouse 0))
      (:else))))

(fn ConstructionScript)