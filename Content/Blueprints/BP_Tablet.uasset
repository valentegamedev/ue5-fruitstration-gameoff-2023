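; BP_Tablet is an in-world tablet actor that displays the player's current order on a WBP_Tablet widget component.
; On BeginPlay it caches the cast widget, waits one tick, then calls ShowOrder to push the game mode's current order and its one-based number to the widget.
; UpdateOrder, not called within this Blueprint, marks the game mode's checked indexes as done on the widget.
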(event EventBeginPlay
  (bind _aswbp_tablet (Utilities|Casting|CastToWBP_Tablet (UserInterface|GetWidget (Variables|Default|GetWidgetComponent))))
  (Variables|Default|SetWidget _aswbp_tablet)
  (Utilities|FlowControl|DelayUntilNextTick)
  (CallFunction|ShowOrder))

(event Collision|EventActorBeginOverlap
  (params (OtherActor :type Actor%20Object%20Reference)))

(event EventTick
  (params (DeltaSeconds :type Float%20%28single-precision%29)))

(fn ConstructionScript)

(fn ShowOrder
  (bind (_order _index) (Default|GetCurrentOrder (CallFunction|GetCastedGameMode)))
  (Default|ShowOrder (Variables|Default|GetWidget) _order (+ _index 1)))

(fn UpdateOrder
  (bind _checkedindexes (Default|GetCheckedIndexes (CallFunction|GetCastedGameMode)))
  (Default|MarkIndexesasDone (Variables|Default|GetWidget) _checkedindexes))