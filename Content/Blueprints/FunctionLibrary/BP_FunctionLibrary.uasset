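; Blueprint function library of shortcut getters for the game's core framework objects.
; It returns the game mode, the first player's HUD and the first player's pawn, cast to BP_GameMode, BP_HUD and BP_CameraPawn.
; The tutorial manager getter finds the BP_TutorialManager actor in the level with GetActorOfClass.
; Failed casts are not handled, and no result is cached.
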(fn GetCastedGameMode
  (bind _asbp_game_mode (Utilities|Casting|CastToBP_GameMode (Game|GetGameMode))
    (:then
      _)
    (:CastFailed
      _))
  (return _asbp_game_mode))

(fn GetCastedHUD
  (bind _asbp_hud (Utilities|Casting|CastToBP_HUD (HUD|GetHUD (Game|GetPlayerController 0)))
    (:then
      _)
    (:CastFailed
      _))
  (return _asbp_hud))

(fn GetTutorialManager
  (bind _returnvalue (Actor|GetActorOfClass 0 "/Game/Blueprints/Tutorial/BP_TutorialManager.BP_TutorialManager_C"))
  (return _returnvalue))

(fn GetCastedPlayerPawn
  (bind _asbp_camera_pawn (Utilities|Casting|CastToBP_CameraPawn (Game|Player|GetPlayerPawn 0))
    (:then
      _)
    (:CastFailed
      _))
  (return _asbp_camera_pawn))