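; BP_Scale is a scale that weighs fruit resting in its box trigger and has a widget for a digit readout.
; Overlap begin and end events add or subtract each VFruit's volume from TotalWeight, treating volume as weight.
; BeginPlay caches the WBP_ScaleDigits widget, and the UpdateDigits event writes a given value to it, though nothing in this graph calls that event.
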(event OnComponentBeginOverlap(BoxComponent)
  (params (OverlappedComponent :type Primitive%20Component%20Object%20Reference) (OtherActor :type Actor%20Object%20Reference) (OtherComp :type Primitive%20Component%20Object%20Reference) (OtherBodyIndex :type Integer) (bFromSweep :type Boolean) (SweepResult :type Hit%20Result%20Structure%20%28by%20ref%29))
  (bind _asvfruit (Utilities|Casting|CastToVFruit OtherActor))
  (bind _returnvalue (Class|VFruit|GetVolume _asvfruit))
  (Variables|Default|SetTotalWeight (+ (Variables|Default|GetTotalWeight) _returnvalue)))

(event OnComponentEndOverlap(BoxComponent)
  (params (OverlappedComponent :type Primitive%20Component%20Object%20Reference) (OtherActor :type Actor%20Object%20Reference) (OtherComp :type Primitive%20Component%20Object%20Reference) (OtherBodyIndex :type Integer))
  (bind _asvfruit (Utilities|Casting|CastToVFruit OtherActor))
  (bind _returnvalue (Class|VFruit|GetVolume _asvfruit))
  (Variables|Default|SetTotalWeight (- (Variables|Default|GetTotalWeight) _returnvalue)))

(event EventUpdateDigits
  (params (NewValue :type Text%20%28by%20ref%29))
  (bind _scaledigits (Variables|Default|GetScaleDigits)
    (:then
      (Default|SetText _scaledigits NewValue))
    (:else)))

(event EventBeginPlay
  (|CallParentFunction)
  (bind _aswbp_scale_digits (Utilities|Casting|CastToWBP_ScaleDigits (UserInterface|GetWidget (Variables|Default|GetDigitsWidget))))
  (Variables|Default|SetScaleDigits _aswbp_scale_digits))

(fn ConstructionScript)