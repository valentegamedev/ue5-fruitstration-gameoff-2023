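; BP_Blade is the blade Blueprint of a fruit-cutting game, handling the feedback played when a fruit is cut.
; PlayEffects spawns Niagara sparks and a BP_Decal, both tinted with the fruit's splash color, then plays a cut sound and a camera shake scaled by the length of the cut direction.
; It then fires an OnFruitCut event, noted as a small hack for the tutorial.
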(event EventPlayEffects
  (params (FruitData :type V%20Fruit%20Data%20Object%20Reference) (Location :type Vector :default "0, 0, 0") (Rotation :type Rotator :default "0, 0, 0") (RawDirection :type Vector :default "0, 0, 0"))
  (bind _splashcolor (Variables|/Script/Fruitstration.VFruitData|GetSplashColor FruitData))
  (Utilities|FlowControl|Sequence
    (:then_0
      (bind _returnvalue (Niagara|SpawnSystematLocation "/Game/Particles/NS_Sparks.NS_Sparks" Location Rotation))
      (Niagara|SetNiagaraVariable(LinearColor) _returnvalue "User.SplashColor" _splashcolor)
      (Game|SpawnActorfromClass "/Game/Blueprints/BP_Decal.BP_Decal_C" (Math|Transform|MakeTransform Location Rotation "1.000000,1.000000,1.000000") "Undefined" "MultiplyWithRoot" 0 _splashcolor 0)
      (CameraShakes|StartCameraShake (Game|GetPlayerCameraManager 0) "/Game/Blueprints/BP_CameraShake.BP_CameraShake_C" (* (Math|Vector|VectorLength RawDirection) 0.45) "CameraLocal" "0, 0, 0")
      (Audio|PlaySound2D "/Game/Sounds/SC_Cut.SC_Cut" 1.0 1.0 0.0 0 0 false))
    (:then_1
      ;[1 1 1] Small hack for the tutorial :)
      (Default|CallOnFruitCutEvent))))

(fn ConstructionScript)