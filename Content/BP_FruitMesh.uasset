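; Geometry Script test actor that converts procedural mesh data into a dynamic mesh.
; Construction builds a box in the DynamicMeshComponent, then BeginPlay resets it and copies in a single triangle created on the ProceduralMesh.
; The P key prints the dynamic mesh's volume for debugging.
; Box boolean subtraction, convex-hull collision generation and physics launch nodes are present but unconnected, so they never run.
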(event Collision|EventActorBeginOverlap
  (params (OtherActor :type Actor%20Object%20Reference)))

(event EventTick
  (params (DeltaSeconds :type Float%20%28single-precision%29)))

(event EventBeginPlay
  (bind _proceduralmesh (Variables|Default|GetProceduralMesh))
  (Utilities|FlowControl|Sequence
    (:then_0
      (Class|ProceduralMeshComponent|CreateMeshSectionLinearColor _proceduralmesh 0 (Utilities|Array|MakeArray "100.000000,0.000000,0.000000" "100.000000,0.000000,100.000000" "0, 0, 0") (Utilities|Array|MakeArray 0 1 2) 0 0 0 0 0 0 0 false false))
    (:then_1
      (bind _returnvalue (DynamicMeshComponent|GetDynamicMesh (Variables|DynamicMeshActor|GetDynamicMeshComponent)))
      (DynamicMesh|Reset _returnvalue)
      (bind _vertices (Class|KismetProceduralMeshLibrary|GetSectionfromProceduralMesh _proceduralmesh))
      (Class|GeometryScriptLibraryMeshBasicEditFunctions|AppendBufferstoMesh _returnvalue (Utilities|Struct|MakeGeometryScriptSimpleMeshBuffers _vertices 0 0 0 0 0 0 0 0 0 0 (Utilities|Array|MakeArray (Utilities|Struct|MakeIntVector 0 1 2))) 0 false 0))))

(event Input|KeyboardEvents|P
  (params (Key :type Key%20Structure :default "None"))
  (:Pressed
    (Development|PrintString "Hello")
    (bind _returnvalue (DynamicMeshComponent|GetDynamicMesh (Variables|DynamicMeshActor|GetDynamicMeshComponent)))
    (Development|PrintString "Volume")
    (Development|PrintString (Utilities|String|ToString(Float) (.Volume (Class|GeometryScriptLibraryMeshQueryFunctions|GetMeshVolumeArea _returnvalue))))))

(fn ConstructionScript
  (bind _returnvalue (DynamicMeshComponent|GetDynamicMesh (Variables|DynamicMeshActor|GetDynamicMeshComponent)))
  (bind _returnvalue_2 (DynamicMesh|Reset _returnvalue))
  (bind _returnvalue_3 (Class|GeometryScriptLibraryMeshPrimitiveFunctions|AppendBox :TargetMesh _returnvalue_2 :Debug 0)))